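; Player controller that runs an initiative-based turn order over all BP_Char actors by possessing each in turn.
; On BeginPlay it selection-sorts them by Ini, highest first, possesses the first and creates the UICharData widget.
; NextPlayer or Tab possesses the next character in the remaining-turn queue and retargets the widget, refilling the queue from the sorted list when empty.
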(event Custom|NextPlayer
  (if (> (Utilities|Array|Length (Variables|Default|GetPlayersInTurn)) 0)
    _
    (else
      (Variables|Default|SetPlayersInTurn (Variables|Default|GetSortedPlayers))))
  (CallFunction|ToNextCharFunc (Variables|Default|GetPlayersInTurn)))

(event EventBeginPlay
  (bind _outactors (Actor|GetAllActorsOfClass "/Game/Blueprint_Prototype/Core/BP_Char.BP_Char_C"))
  (bind _output_get (Variables|Default|SetPlayers _outactors))
  (bind _output_get_2 (Variables|Default|SetAmount (Utilities|Array|Length _output_get)))
  (Development|PrintString (Utilities|String|ToString(Integer) _output_get_2))
  (bind _resultarray (CallFunction|SortArray (Variables|Default|GetPlayers)))
  (bind _output_get_3 (Variables|Default|SetSortedPlayers _resultarray))
  (bind _output_get_4 (Variables|Default|SetPlayers _output_get_3))
  (bind _output_get_5 (Variables|Default|SetPlayersInTurn _output_get_4))
  (bind _output_get_6 (Variables|Default|SetCurPlayer (Utilities|Array|Get(acopy) _output_get_5)))
  (Pawn|UnPossess)
  (Pawn|Possess _output_get_6)
  (Utilities|Array|RemoveItem _output_get_5 _output_get_6)
  (bind _returnvalue (UserInterface|CreateWidget "/Game/Blueprint_Prototype/Core/UICharData.UICharData_C" self _output_get_6))
  (UserInterface|Viewport|AddtoViewport _returnvalue 0)
  (bind _output_get_7 (Variables|Default|SetUI _returnvalue))
  (Variables|/Game/Blueprint_Prototype/Core/BP_Char.BP_Char_C|SetUI _output_get_6 _output_get_7))

(event Input|KeyboardEvents|Tab
  (params (Key :type Key%20Structure :default "None"))
  (:Pressed
    (if (> (Utilities|Array|Length (Variables|Default|GetPlayersInTurn)) 0)
      _
      (else
        (Variables|Default|SetPlayersInTurn (Variables|Default|GetSortedPlayers))))
    (CallFunction|ToNextCharFunc (Variables|Default|GetPlayersInTurn))))

(fn ConstructionScript)

(fn SortArray
  (params (BaseArray :type Array%20of%20BP%20Char%20Object%20References))
  (bind _tarr (LocalVariables|GetTArr))
  (for _index (range 0 (- (Variables|Default|GetAmount) 1))
    (LocalVariables|Setmax 9999)
    (bind (_array_element _array_index) (Utilities|Array|ForEachLoopwithBreak BaseArray)
      (:LoopBody
        (if (< (.ini (.params (Variables|/Game/Blueprint_Prototype/Core/BP_Char.BP_Char_C|GetCharData _array_element))) (LocalVariables|Getmax))
          (LocalVariables|Setmax (.ini (.params (Variables|/Game/Blueprint_Prototype/Core/BP_Char.BP_Char_C|GetCharData _array_element))))
          (LocalVariables|SetminId _array_index)))
      (:Completed
        (Utilities|Array|Add (LocalVariables|GetTArr) (Utilities|Array|Get(acopy) BaseArray (LocalVariables|GetminId)))
        (Utilities|Array|RemoveIndex BaseArray (LocalVariables|GetminId)))))
  (Utilities|Array|Reverse _tarr)
  (CallFunction|PrintChars _tarr)
  (return _tarr))

(fn PrintChars
  (params (Array :type Array%20of%20BP%20Char%20Object%20References))
  (for _array_element Array
    (Development|PrintString (Utilities|String|Append (.name (.params (Variables|/Game/Blueprint_Prototype/Core/BP_Char.BP_Char_C|GetCharData _array_element))) (Utilities|String|ToString(Integer) (.ini (.params (Variables|/Game/Blueprint_Prototype/Core/BP_Char.BP_Char_C|GetCharData _array_element))))) true true "(R=0.000000,G=0.660000,B=1.000000,A=1.000000)" 1e+01)))

(fn ToNextCharFunc
  (params (InputPin :type Array%20of%20BP%20Char%20Object%20References))
  (bind _output_get (Variables|Default|SetCurPlayer (Utilities|Array|Get(acopy) InputPin)))
  (Pawn|UnPossess)
  (Pawn|Possess _output_get)
  (Utilities|Array|RemoveItem InputPin _output_get)
  (Variables|/Game/Blueprint_Prototype/Core/UICharData.UICharData_C|SetChar (Variables|Default|GetUI) _output_get))