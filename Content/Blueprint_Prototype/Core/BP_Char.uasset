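; Prototype player character for turn-based, step-by-step movement, where each move spends an action point.
; CalcRotation snaps control yaw to quarter turns on an arrow, and WASD input maps against the facing to rotate the cube.
; A timeline lerps the cube's location with input disabled, then decrements AP or resets it and calls NextPlayer on the player controller.
; A timeline-based smooth rotation helper exists but is never run.
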(event EventBeginPlay
  (Variables|Default|SetGM (Game|GetGameMode))
  (bind _aspc_base (Utilities|Casting|CastToPC_Base (Game|GetPlayerController 0)))
  (Variables|Default|SetPC _aspc_base)
  (Variables|Default|SetStartLoc (Transformation|GetWorldLocation (Variables|Default|GetCube)))
  (Variables|Default|SetCharData (Utilities|Struct|MakeCharData (.params (Variables|Default|GetCharData)))))

(event Input|AxisEvents|InputAxisMouse_X
  (params (AxisValue :type Float%20%28single-precision%29))
  (Pawn|Input|AddControllerYawInput AxisValue)
  (CallFunction|CalcRotation))

(event Input|AxisEvents|InputAxisForward
  (params (AxisValue :type Float%20%28single-precision%29))
  (bind _returnvalue (Game|GetPlayerController 0))
  (bind _cube (Variables|Default|GetCube))
  (bind _cube_2 (Variables|Default|GetCube))
  (bind _step (Variables|Default|GetStep))
  (bind _returnvalue_2 (* "" _step))
  (switch int (Math|Float|Truncate AxisValue)
    (:-1
      (Development|PrintString "S")
      (switch Utilities|FlowControl|Switch|SwitchonECameraDirection "NewEnumerator0"
        (:NewEnumerator0
          (Variables|Default|SetCharData (Utilities|Struct|MakeCharData (.params (Variables|Default|GetCharData))) :!label _label)
          (Transformation|SetWorldRotation _cube_2 "0.000000,-180.000000, 0" false false))
        (:NewEnumerator1
          (Variables|Default|SetCharData (Utilities|Struct|MakeCharData (.params (Variables|Default|GetCharData))) :!label _label_2)
          (Transformation|SetWorldRotation _cube "0,-90.000000, 0" false false))
        (:NewEnumerator2
          (Variables|Default|SetCharData (Utilities|Struct|MakeCharData (.params (Variables|Default|GetCharData))) :!label _label_3)
          (Transformation|SetWorldRotation _cube_2 "0, 0, 0" false false))
        (:NewEnumerator3
          (Variables|Default|SetCharData (Utilities|Struct|MakeCharData (.params (Variables|Default|GetCharData))) :!label _label_4)
          (Transformation|SetWorldRotation _cube "0.000000,90.000000,0.000000" false false))))
    (:1
      (Development|PrintString "W")
      (switch Utilities|FlowControl|Switch|SwitchonECameraDirection "NewEnumerator0"
        (:NewEnumerator0
          (goto _label_3))
        (:NewEnumerator1
          (goto _label_4))
        (:NewEnumerator2
          (goto _label))
        (:NewEnumerator3
          (goto _label_2)))))
  (Input|DisableInput _returnvalue)
  (CallFunction|CalcRotation)
  (bind _way (Timeline|Timeline_0 PlayFromStart)
    (:Update
      (Transformation|SetWorldLocation (Variables|Default|GetCube) (Math|Vector|Lerp(Vector) (Variables|Default|GetStartLoc) (Math|Vector|MakeVector (+ (.x (Variables|Default|GetStartLoc)) (.x _returnvalue_2)) (+ (.y (Variables|Default|GetStartLoc)) (.y _returnvalue_2)) (.z (Variables|Default|GetStartLoc))) _way) false false))
    (:Finished
      (Variables|Default|SetStartLoc (Math|Vector|MakeVector (+ (.x (Variables|Default|GetStartLoc)) (.x _returnvalue_2)) (+ (.y (Variables|Default|GetStartLoc)) (.y _returnvalue_2)) (.z (Variables|Default|GetStartLoc))))
      (Input|EnableInput _returnvalue)
      (if (> (.ap (.params (Variables|Default|GetCharData))) 1)
        (Variables|Default|SetCharData (Utilities|Struct|MakeCharData (Utilities|Struct|MakeSCharParameters (.name (.params (Variables|Default|GetCharData))) (.hp (.params (Variables|Default|GetCharData))) (.mp (.params (Variables|Default|GetCharData))) (- (.ap (.params (Variables|Default|GetCharData))) 1) (.xp (.params (Variables|Default|GetCharData))) (.sp (.params (Variables|Default|GetCharData))) (.ini (.params (Variables|Default|GetCharData))) (.thumbnail (.params (Variables|Default|GetCharData))) (.class (.params (Variables|Default|GetCharData))))))
        (else
          (Variables|Default|SetCharData (Utilities|Struct|MakeCharData (Utilities|Struct|MakeSCharParameters (.name (.params (Variables|Default|GetCharData))) (.hp (.params (Variables|Default|GetCharData))) (.mp (.params (Variables|Default|GetCharData))) 3 (.xp (.params (Variables|Default|GetCharData))) (.sp (.params (Variables|Default|GetCharData))) (.ini (.params (Variables|Default|GetCharData))) (.thumbnail (.params (Variables|Default|GetCharData))) (.class (.params (Variables|Default|GetCharData))))))
          (Default|NextPlayer (Variables|Default|GetPC)))))))

(event Input|AxisEvents|InputAxisRight
  (params (AxisValue :type Float%20%28single-precision%29))
  (bind _returnvalue (Game|GetPlayerController 0))
  (bind _cube (Variables|Default|GetCube))
  (bind _cube_2 (Variables|Default|GetCube))
  (bind _step (Variables|Default|GetStep))
  (bind _returnvalue_2 (* "" _step))
  (switch int (Math|Float|Truncate AxisValue)
    (:-1
      (Development|PrintString "A")
      (switch Utilities|FlowControl|Switch|SwitchonECameraDirection "NewEnumerator0"
        (:NewEnumerator0
          (Variables|Default|SetCharData (Utilities|Struct|MakeCharData (.params (Variables|Default|GetCharData))) :!label _label)
          (Transformation|SetWorldRotation _cube "0,-90.000000, 0" false false))
        (:NewEnumerator1
          (Variables|Default|SetCharData (Utilities|Struct|MakeCharData (.params (Variables|Default|GetCharData))) :!label _label_2)
          (Transformation|SetWorldRotation _cube_2 "0, 0, 0" false false))
        (:NewEnumerator2
          (Variables|Default|SetCharData (Utilities|Struct|MakeCharData (.params (Variables|Default|GetCharData))) :!label _label_3)
          (Transformation|SetWorldRotation _cube "0.000000,90.000000,0.000000" false false))
        (:NewEnumerator3
          (Variables|Default|SetCharData (Utilities|Struct|MakeCharData (.params (Variables|Default|GetCharData))) :!label _label_4)
          (Transformation|SetWorldRotation _cube_2 "0.000000,-180.000000, 0" false false))))
    (:1
      (Development|PrintString "D")
      (switch Utilities|FlowControl|Switch|SwitchonECameraDirection "NewEnumerator0"
        (:NewEnumerator0
          (goto _label_3))
        (:NewEnumerator1
          (goto _label_4))
        (:NewEnumerator2
          (goto _label))
        (:NewEnumerator3
          (goto _label_2)))))
  (Input|DisableInput _returnvalue)
  (CallFunction|CalcRotation)
  (bind _way (Timeline|Timeline_0 PlayFromStart)
    (:Update
      (Transformation|SetWorldLocation (Variables|Default|GetCube) (Math|Vector|Lerp(Vector) (Variables|Default|GetStartLoc) (Math|Vector|MakeVector (+ (.x (Variables|Default|GetStartLoc)) (.x _returnvalue_2)) (+ (.y (Variables|Default|GetStartLoc)) (.y _returnvalue_2)) (.z (Variables|Default|GetStartLoc))) _way) false false))
    (:Finished
      (Variables|Default|SetStartLoc (Math|Vector|MakeVector (+ (.x (Variables|Default|GetStartLoc)) (.x _returnvalue_2)) (+ (.y (Variables|Default|GetStartLoc)) (.y _returnvalue_2)) (.z (Variables|Default|GetStartLoc))))
      (Input|EnableInput _returnvalue)
      (if (> (.ap (.params (Variables|Default|GetCharData))) 1)
        (Variables|Default|SetCharData (Utilities|Struct|MakeCharData (Utilities|Struct|MakeSCharParameters (.name (.params (Variables|Default|GetCharData))) (.hp (.params (Variables|Default|GetCharData))) (.mp (.params (Variables|Default|GetCharData))) (- (.ap (.params (Variables|Default|GetCharData))) 1) (.xp (.params (Variables|Default|GetCharData))) (.sp (.params (Variables|Default|GetCharData))) (.ini (.params (Variables|Default|GetCharData))) (.thumbnail (.params (Variables|Default|GetCharData))) (.class (.params (Variables|Default|GetCharData))))))
        (else
          (Variables|Default|SetCharData (Utilities|Struct|MakeCharData (Utilities|Struct|MakeSCharParameters (.name (.params (Variables|Default|GetCharData))) (.hp (.params (Variables|Default|GetCharData))) (.mp (.params (Variables|Default|GetCharData))) 3 (.xp (.params (Variables|Default|GetCharData))) (.sp (.params (Variables|Default|GetCharData))) (.ini (.params (Variables|Default|GetCharData))) (.thumbnail (.params (Variables|Default|GetCharData))) (.class (.params (Variables|Default|GetCharData))))))
          (Default|NextPlayer (Variables|Default|GetPC)))))))

(fn ConstructionScript)

(fn CalcRotation
  (bind _returnvalue (Pawn|GetControlRotation :!class /Script/Engine.Pawn))
  (bind _arrow1 (Variables|Default|GetArrow1))
  (bind _returnvalue_2 (Transformation|GetWorldRotation _arrow1))
  (bind _returnvalue_3 (Math|Float|%(Float) (.yaw _returnvalue) 3.6e+02))
  (bind _returnvalue_4 (+ _returnvalue_3 45.0))
  (bind _returnvalue_5 (/ _returnvalue_4 9e+01))
  (bind _returnvalue_6 (Math|Float|Floor _returnvalue_5))
  (bind _returnvalue_7 (* _returnvalue_6 90))
  (bind _returnvalue_8 (Math|Conversions|ToFloat(Integer) _returnvalue_7))
  ;[1 1 1] Calculating Direction of Character
  (Variables|Default|SetDesiredRotation (Math|Rotator|MakeRotator (.roll _returnvalue_2) (.pitch _returnvalue_2) _returnvalue_8))
  (Transformation|SetWorldRotation _arrow1 (Math|Rotator|MakeRotator (.roll _returnvalue_2) (.pitch _returnvalue_2) _returnvalue_8) false false)
  (switch int _returnvalue_6
    (:Default
      (Variables|Default|SetCharData (Utilities|Struct|MakeCharData (.params (Variables|Default|GetCharData))) :!label _label))
    (:0
      (goto _label))
    (:1
      (Variables|Default|SetCharData (Utilities|Struct|MakeCharData (.params (Variables|Default|GetCharData)))))
    (:2
      (Variables|Default|SetCharData (Utilities|Struct|MakeCharData (.params (Variables|Default|GetCharData)))))
    (:3
      (Variables|Default|SetCharData (Utilities|Struct|MakeCharData (.params (Variables|Default|GetCharData)))))))

(fn RotFunction
  (|RotationTemplate
    (:End
      (return))))