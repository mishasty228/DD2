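; BP_GameMaster is a game master Blueprint that advances to the next character through SetNextChar when N is pressed.
; BeginPlay looks up the TileMap actor but does nothing further with it.
; A disconnected, never-executed chain traces under the mouse cursor, highlights the hit TileBase blue if available or red if not, resets the previous tile, and prints the tile's coordinates and index.
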(event EventBeginPlay
  (Actor|GetActorOfClass "/Script/DD2.TileMap"))

(event Collision|EventActorBeginOverlap
  (params (OtherActor :type Actor%20Object%20Reference)))

(event EventTick
  (params (DeltaSeconds :type Float%20%28single-precision%29)))

(event Input|KeyboardEvents|N
  (params (Key :type Key%20Structure :default "None"))
  (:Pressed
    (Class|GameMaster|SetNextChar)))

(fn ConstructionScript)