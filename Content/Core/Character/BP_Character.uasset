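; Character Blueprint that spawns as a randomized hero with its own type, gear, stats, actions, thumbnail and name.
; On BeginPlay, Initialize picks a random entry from Types, copies its data into variables, and sets the weapon mesh and a random chest armor variation.
; Weapon damage and armor bonuses are then added onto the base stats, while the talisman is only stored.
; A MovetoLocation event relays movement targets to the AI controller.
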(event EventBeginPlay
  (CallFunction|Initialize))

(event Collision|EventActorBeginOverlap
  (params (OtherActor :type Actor%20Object%20Reference)))

(event EventTick
  (params (DeltaSeconds :type Float%20%28single-precision%29)))

(event EventMovetoLocation
  (params (Target :type Vector :default "0, 0, 0"))
  (AI|Navigation|MovetoLocation (AI|GetAIController self) Target -1.0 true true false true 0))

(fn ConstructionScript)

(fn Initialize
  (bind _output_get (Variables|Default|SetCharData (.OutItem (Utilities|Array|Random (Variables|Default|GetTypes)))))
  (Variables|Default|SetHeroType (Variables|/Script/DD2.CharDataAsset|GetCharType _output_get))
  (Components|StaticMesh|SetStaticMesh (Variables|Default|GetWeaponMesh) (Variables|/Script/DD2.WeaponItemDataAsset|GetWeaponMesh (Variables|/Script/DD2.CharDataAsset|GetWeapon (Variables|Default|GetCharData))))
  (Variables|Default|SetWeapon (Variables|/Script/DD2.CharDataAsset|GetWeapon (Variables|Default|GetCharData)))
  (Class|SkinnedMeshComponent|SetSkeletalMesh (Variables|Default|GetClothesMesh) (.OutItem (Utilities|Array|Random (Variables|/Script/DD2.ArmorDataAsset|GetChestMeshVariations (Variables|/Script/DD2.CharDataAsset|GetArmor (Variables|Default|GetCharData))))) true)
  (Variables|Default|SetArmor (Variables|/Script/DD2.CharDataAsset|GetArmor (Variables|Default|GetCharData)))
  (Variables|Default|SetTalisman (Variables|/Script/DD2.CharDataAsset|GetTalisman (Variables|Default|GetCharData)))
  (Variables|Default|SetActions (Variables|/Script/DD2.CharDataAsset|GetActions (Variables|Default|GetCharData)))
  (Variables|Default|SetHealthPoints (Variables|/Script/DD2.CharDataAsset|GetHealthPoints (Variables|Default|GetCharData)))
  (Variables|Default|SetDamagePoints (Variables|/Script/DD2.CharDataAsset|GetDamagePoints (Variables|Default|GetCharData)))
  (Variables|Default|SetActionPoints (Variables|/Script/DD2.CharDataAsset|GetActionPoints (Variables|Default|GetCharData)))
  (Variables|Default|SetSpeedPoints (Variables|/Script/DD2.CharDataAsset|GetSpeedPoints (Variables|Default|GetCharData)))
  (Variables|Default|SetDamageResist (Variables|/Script/DD2.CharDataAsset|GetDamageResist (Variables|Default|GetCharData)))
  (Variables|Default|SetDodgeChance (Variables|/Script/DD2.CharDataAsset|GetDodgeChance (Variables|Default|GetCharData)))
  (Variables|Default|SetFireResist (Variables|/Script/DD2.CharDataAsset|GetFireResist (Variables|Default|GetCharData)))
  (Variables|Default|SetIceResist (Variables|/Script/DD2.CharDataAsset|GetIceResist (Variables|Default|GetCharData)))
  (Variables|Default|SetPoiseResist (Variables|/Script/DD2.CharDataAsset|GetPoiseResist (Variables|Default|GetCharData)))
  (Variables|Default|SetBleedResist (Variables|/Script/DD2.CharDataAsset|GetBleedResist (Variables|Default|GetCharData)))
  (Variables|Default|SetStunResist (Variables|/Script/DD2.CharDataAsset|GetStunResist (Variables|Default|GetCharData)))
  (Variables|Default|SetThumbnail (Variables|/Script/DD2.CharDataAsset|GetThumbnail (Variables|Default|GetCharData)))
  (Variables|Default|SetName (.OutItem (Utilities|Array|Random (Variables|Default|GetNames))))
  (CallFunction|AddWeaponParams (Variables|Default|GetWeapon))
  (CallFunction|AddArmorParams (Variables|Default|GetArmor)))

(fn AddWeaponParams
  (params (Weapon :type Weapon%20Item%20Data%20Asset%20Object%20Reference))
  (Variables|Default|SetDamagePoints (+ (Variables|Default|GetDamagePoints) (Variables|/Script/DD2.WeaponItemDataAsset|GetDamage Weapon)))
  (return))

(fn AddArmorParams
  (params (ArmorVar :type Armor%20Data%20Asset%20Object%20Reference))
  (Variables|Default|SetHealthPoints (+ (Variables|Default|GetHealthPoints) (Variables|/Script/DD2.ArmorDataAsset|GetHealth ArmorVar)))
  (Variables|Default|SetSpeedPoints (+ (Variables|Default|GetSpeedPoints) (Variables|/Script/DD2.ArmorDataAsset|GetSpeed ArmorVar)))
  (Variables|Default|SetDamageResist (+ (Variables|Default|GetDamageResist) (Variables|/Script/DD2.ArmorDataAsset|GetDamageResist ArmorVar)))
  (Variables|Default|SetDodgeChance (+ (Variables|Default|GetDodgeChance) (Variables|/Script/DD2.ArmorDataAsset|GetDodgeChance ArmorVar)))
  (Variables|Default|SetFireResist (+ (Variables|Default|GetFireResist) (Variables|/Script/DD2.ArmorDataAsset|GetFireResist ArmorVar)))
  (Variables|Default|SetIceResist (+ (Variables|Default|GetIceResist) (Variables|/Script/DD2.ArmorDataAsset|GetIceResist ArmorVar)))
  (Variables|Default|SetPoiseResist (+ (Variables|Default|GetPoiseResist) (Variables|/Script/DD2.ArmorDataAsset|GetPoiseResist ArmorVar)))
  (Variables|Default|SetBleedResist (+ (Variables|Default|GetBleedResist) (Variables|/Script/DD2.ArmorDataAsset|GetBleedResist ArmorVar)))
  (Variables|Default|SetStunResist (+ (Variables|Default|GetStunResist) (Variables|/Script/DD2.ArmorDataAsset|GetStunResist ArmorVar))))