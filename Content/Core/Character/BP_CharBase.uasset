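; BP_CharBase is a character Blueprint, apparently a base class, that randomizes its character data at spawn.
; On BeginPlay it picks a random ECharType, using an inclusive range from zero to the enum's entry count, and passes it to CharDataComponent to generate that type's parameters.
; The construction script is empty, with a disconnected copy of the same randomization, and overlap and Tick events are disabled.
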(event EventBeginPlay
  (Class|CharDataComponent|GenerateRandomParametersforType (Variables|Default|GetCharDataComponent) (Utilities|Enum|ByteToEnumECharType (Math|Conversions|ToByte(Integer) (Math|Random|RandomIntegerinRange 0 (|GetNumEnumEntries))))))

(event Collision|EventActorBeginOverlap
  (params (OtherActor :type Actor%20Object%20Reference)))

(event EventTick
  (params (DeltaSeconds :type Float%20%28single-precision%29)))

(fn ConstructionScript)