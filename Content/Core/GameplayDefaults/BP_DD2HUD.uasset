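; BP_DD2HUD is a HUD Blueprint that relays character updates and inventory visibility requests to the UI_HUD widget.
; It casts the HUD reference to UI_HUD, then calls UpdateHUD with the given character or ShowEquipment with the show flag.
; BeginPlay only calls its parent.
; Disconnected nodes for filling UI_Inventory slots and printing a debug string never run.
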(event EventBeginPlay
  (|CallParentFunction))

(event EventShowInventoryWidget
  (params (Show :type Boolean))
  (bind _asui_hud (Utilities|Casting|CastToUI_HUD (Variables|Default|GetHUD)))
  (Default|ShowEquipment _asui_hud Show))

(fn ConstructionScript)

(fn UpdateHUD
  (params (Char :type Char%20Base%20Object%20Reference))
  (bind _asui_hud (Utilities|Casting|CastToUI_HUD (Variables|Default|GetHUD)))
  (Default|UpdateHUD _asui_hud Char))